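; A bonfire actor that serves as a save point when the player interacts with it.
; Interacting sets FireActive, asks the GRGameModeBase game mode to write the save game, prints a confirmation message, then lights the flames.
; On load, UpdateFlames reactivates the particle system if the fire was already active.
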(event Custom|UpdateFlames
  ;[1 1 1] Enables flames
  (if (Variables|Default|GetbFireActive)
    (Components|Activation|Activate (Variables|Default|GetParticleSystem) false)))

(event EventInteract
  (params (InstigationPawn :type Pawn%20Object%20Reference))
  ;[1 1 1] Save Game
  (Variables|Default|SetbFireActive true)
  (bind _asgrgame_mode_base (Utilities|Casting|CastToGRGameModeBase (Game|GetGameMode)))
  (Class|GRGameModeBase|WriteSaveGame _asgrgame_mode_base)
  (Development|PrintString "Bonfire World Saved" true true "(R=0.500000,G=0.072123,B=0.488862,A=1.000000)")
  (CallFunction|UpdateFlames))

(event EventOnActorLoaded
  (CallFunction|UpdateFlames))

(fn ConstructionScript)