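; Treasure chest Blueprint that handles pawn interaction by passing it to the parent class's Interact and printing a debug message.
; Older Blueprint logic is left disconnected and never runs: a FlipFlop lid timeline with a particle effect on opening, and a LidOpened debug print.
; A keycard gameplay-tag check on GRActionComponent is also unwired, noted as deferred for replication.
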(event EventTick
  (params (DeltaSeconds :type Float%20%28single-precision%29)))

(event EventInteract
  (params (InstigationPawn :type Pawn%20Object%20Reference))
  ;[1 1 1] Open Lid
  (|CallParentFunction InstigationPawn)
  (Development|PrintString "TreasureChest Interact (BP)" true true "(R=0.000000,G=0.660000,B=1.000000,A=1.000000)" 5.0))

(fn ConstructionScript)