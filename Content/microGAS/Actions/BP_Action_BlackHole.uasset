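; BP_Action_BlackHole is a Black Hole action Blueprint that costs Rage to use.
; CanStart runs the parent check, then requires the instigator's attribute Rage to meet RageCost, printing an on-screen warning when it falls short.
; StartAction deducts RageCost from those attributes before calling the parent StartAction, which handles the rest of the action.
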(event EventStartAction
  (params (Instigator :type Actor%20Object%20Reference))
  (bind _returnvalue (Class|GRAttributeComponent|GetAttributes Instigator))
  (Class|GRAttributeComponent|ApplyRage _returnvalue Instigator (/ (Variables|Default|GetRageCost) -1.0))
  (|CallParentFunction Instigator))

(fn CanStart
  (params (Instigator :type Actor%20Object%20Reference))
  (bind _returnvalue (|CallParentFunction Instigator))
  (if _returnvalue
    (bind _returnvalue_2 (Class|GRAttributeComponent|GetAttributes Instigator))
    (if (>= (Class|GRAttributeComponent|GetRage _returnvalue_2) (Variables|Default|GetRageCost))
      (return true)
      (else
        (Development|PrintString "Not Enough Rage" true true "(R=1.000000,G=0.250000,B=0.000000,A=1.000000)")
        (return false)))
    (else
      (return false))))